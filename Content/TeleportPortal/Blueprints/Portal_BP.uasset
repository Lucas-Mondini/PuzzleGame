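; Portal actor that displays the view from its linked portal's capture camera on its plane.
; On BeginPlay it creates a dynamic instance of Portal_MAT and a viewport-sized render target, feeds the target into the material, and assigns it as the linked portal camera's output.
; Its tick group is set to PostUpdateWork, though Tick and overlap events are empty, so no teleport or camera-tracking logic exists here.
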(event EventBeginPlay
  (bind _returnvalue (Viewport|GetViewportSize))
  (Components|Tick|SetTickGroup "TG_PostUpdateWork")
  (bind _returnvalue_2 (Rendering|Material|CreateDynamicMaterialInstance "/Game/TeleportPortal/Blueprints/Portal_MAT.Portal_MAT" "None" "None" :!class /Script/Engine.KismetMaterialLibrary))
  (bind _output_get (Variables|Default|SetPortal_MAT _returnvalue_2))
  (Rendering|Material|SetMaterial (Variables|Default|GetPortalPlane) 0 _output_get)
  (bind _returnvalue_3 (Rendering|CreateRenderTarget2D (Math|Float|Truncate (.x _returnvalue)) (Math|Float|Truncate (.y _returnvalue)) "RTF_RGBA16f"))
  (bind _output_get_2 (Variables|Default|SetPortal_RT _returnvalue_3))
  (Rendering|Material|SetTextureParameterValue (Variables|Default|GetPortal_MAT) "Texture" _output_get_2)
  (Variables|/Script/Engine.SceneCaptureComponent2D|SetTextureTarget (Variables|Portal_BP_C|GetPortalCamera (Variables|Default|GetLinked%20Portal)) (Variables|Default|GetPortal_RT)))

(event Collision|EventActorBeginOverlap
  (params (OtherActor :type Actor%20Object%20Reference)))

(event EventTick
  (params (DeltaSeconds :type Float%20%28single-precision%29)))

(fn ConstructionScript)